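; Main player controller for the loop game, handling the splash screen, HUD and mouse selection of world actors.
; On BeginPlay it shows the HUD if the game instance says the game has started, otherwise the splash widget until the StartGame event fires.
; Left click traces under the cursor, messaging actors implementing I_Selectable on press and again on release.
; Input actions also take high-res screenshots and quit the game.
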(event Custom|CustomEvent_0
  (CallFunction|SetHud))

(event EventBeginPlay
  (bind _asgi_loop_game (Utilities|Casting|CastToGI_LoopGame (Game|GetGameInstance)))
  (if (Variables|/Game/LD47Custom/Blueprints/Logic/GI_LoopGame.GI_LoopGame_C|GetGameStarted _asgi_loop_game)
    (CallFunction|SetHud)
    (else
      (CallFunction|SetSplash)
      (EventDispatchers|BindEventtoStartGame _asgi_loop_game (delegate Custom|CustomEvent_0)))))

(event EventTick
  (params (DeltaSeconds :type Float%20%28single-precision%29)))

(event Input|ActionEvents|InputActionScreenShot
  (params (Key :type Key%20Structure :default "None"))
  (:Pressed
    (Class|AutomationBlueprintFunctionLibrary|TakeHighResScreenshot 1024 1024 "" 0)))

(event Input|ActionEvents|InputActionExit
  (params (Key :type Key%20Structure :default "None"))
  (:Pressed
    (Game|QuitGame 0 "Quit" false)))

(event Input|MouseEvents|LeftMouseButton
  (params (Key :type Key%20Structure :default "None"))
  (bind _returnvalue (Game|GetPlayerController 0))
  (bind (_worldlocation _worlddirection) (Game|Player|ConvertMouseLocationToWorldSpace _returnvalue))
  (:Pressed
    (bind _outhit (Collision|LineTraceByChannel _worldlocation (+ _worldlocation (* _worlddirection 1e+05)) "TraceTypeQuery1" false 0 "None"))
    (if (Utilities|DoesObjectImplementInterface (.HitActor (Collision|BreakHitResult _outhit)) "/Game/LD47Custom/Blueprints/Logic/i_Selectable.i_Selectable_C")
      (Variables|Default|SetSelectedActor (.HitActor (Collision|BreakHitResult _outhit)))
      (Class|ISelectable|RecieveSelection(Message) (.HitActor (Collision|BreakHitResult _outhit)))))
  (:Released
    (Class|ISelectable|LoseSelection(Message) (Variables|Default|GetSelectedActor))
    (Variables|Default|SetSelectedActor 0)))

(fn ConstructionScript)

(fn SetHud
  (Viewport|RemoveAllWidgets)
  (Input|SetInputModeGameandUI (Game|GetPlayerController 0) 0 "DoNotLock" false)
  (Variables|Default|SetbShowMouseCursor true)
  (bind _returnvalue (UserInterface|CreateWidget "/Game/LD47Custom/UI/wdgt_HUD.wdgt_HUD_C" self))
  (UserInterface|Viewport|AddtoViewport _returnvalue 0))

(fn SetSplash
  (Viewport|RemoveAllWidgets)
  (Variables|Default|SetbShowMouseCursor true)
  (bind _returnvalue (UserInterface|CreateWidget "/Game/LD47Custom/UI/wdgt_Splash.wdgt_Splash_C" self))
  (UserInterface|Viewport|AddtoViewport _returnvalue 0)
  (Input|SetInputModeUIOnly self _returnvalue "DoNotLock"))