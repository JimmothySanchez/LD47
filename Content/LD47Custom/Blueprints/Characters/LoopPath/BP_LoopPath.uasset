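; BP_LoopPath is a movable looping spline path steered by the MoveForward and MoveRight input axes through its movement component.
; On BeginPlay it spawns a BP_LoopCorner at each spline point, passes it the point index and attaches it to itself.
; UpdateSplineMesh rebuilds cylinder spline meshes between neighboring points, wrapping to close the loop, but its construction script call is disconnected.
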(event EventBeginPlay
  (CallFunction|CreateAnchorPoints))

(event Collision|EventActorBeginOverlap
  (params (OtherActor :type Actor%20Object%20Reference)))

(event EventTick
  (params (DeltaSeconds :type Float%20%28single-precision%29)))

(event Input|AxisEvents|InputAxisMoveRight
  (params (AxisValue :type Float%20%28single-precision%29))
  (Class|PawnMovementComponent|AddInputVector (Variables|Default|GetMovementComponent) (Math|Vector|MakeVector 0.0 AxisValue 0.0) false))

(event Input|AxisEvents|InputAxisMoveForward
  (params (AxisValue :type Float%20%28single-precision%29))
  (Class|PawnMovementComponent|AddInputVector (Variables|Default|GetMovementComponent) (Math|Vector|MakeVector AxisValue 0.0 0.0) false))

(fn ConstructionScript)

(fn UpdateSplineMesh
  (bind _returnvalue (Actor|GetComponentsByClass "/Script/Engine.SplineMeshComponent"))
  (bind _spline (Variables|Default|GetSpline))
  (bind _splinewidth (Variables|Default|GetSplineWidth))
  (bind _returnvalue_2 (Spline|GetNumberOfSplinePoints _spline))
  (while (> (Utilities|Array|Length _returnvalue) 0)
    (Components|DestroyComponent (Utilities|Array|Get(acopy) _returnvalue)))
  (for _index (range 1 _returnvalue_2)
    (bind _returnvalue_3 (AddComponent|AddSplineMeshComponent false (Math|Transform|MakeTransform "0, 0, 0")))
    (Transformation|SetMobility _returnvalue_3 "Movable")
    (SplineMesh|SetStartScale _returnvalue_3 (Math|Vector2D|MakeVector2D _splinewidth _splinewidth) false :!class /Script/Engine.SplineMeshComponent)
    (SplineMesh|SetEndScale _returnvalue_3 (Math|Vector2D|MakeVector2D _splinewidth _splinewidth) false :!class /Script/Engine.SplineMeshComponent)
    (SplineMesh|SetStartandEnd _returnvalue_3 (.Location (Spline|GetLocationandTangentatSplinePoint (Variables|Default|GetSpline) _index "World")) (.Tangent (Spline|GetLocationandTangentatSplinePoint (Variables|Default|GetSpline) _index "World")) (.Location (Spline|GetLocationandTangentatSplinePoint (Variables|Default|GetSpline) (Math|Integer|%(Integer) (+ _index 1) _returnvalue_2) "World")) (.Tangent (Spline|GetLocationandTangentatSplinePoint (Variables|Default|GetSpline) (Math|Integer|%(Integer) (+ _index 1) _returnvalue_2) "World")) false :!class /Script/Engine.SplineMeshComponent)
    (Components|StaticMesh|SetStaticMesh _returnvalue_3 "/Game/StarterContent/Shapes/Shape_Cylinder.Shape_Cylinder")
    (SplineMesh|SetForwardAxis _returnvalue_3 "Z" true)
    (Rendering|Material|SetMaterial _returnvalue_3 0 (Variables|Default|GetSplineMat))))

(fn CreateAnchorPoints
  (for _index (range 0 (- (Spline|GetNumberOfSplinePoints (Variables|Default|GetSpline)) 1))
    (LocalVariables|SetCurrentindex _index)
    (bind _returnvalue (Game|SpawnActorfromClass "/Game/LD47Custom/Blueprints/Characters/LoopPath/BP_LoopCorner.BP_LoopCorner_C" (Math|Transform|MakeTransform (Spline|GetLocationatSplinePoint (Variables|Default|GetSpline) (LocalVariables|GetCurrentindex) "World")) "Undefined" 0 (LocalVariables|GetCurrentindex) 0))
    (Transformation|AttachActorToActor _returnvalue self "None" "KeepWorld" "KeepWorld" "KeepWorld" true)))