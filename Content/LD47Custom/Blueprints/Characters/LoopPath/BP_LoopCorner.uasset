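; BP_LoopCorner is a draggable corner handle that reshapes the spline of the player pawn's BP_LoopPath.
; Selection detaches it from that pawn, and deselection reattaches it, both keeping world transform.
; While selected, Tick traces from the mouse cursor, moves the corner to the hit's XY at its current height, and writes that location to its owned spline point.
; It also prints the point index each selected frame.
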(event EventBeginPlay
  (bind _asbp_loop_path (Utilities|Casting|CastToBP_LoopPath (Game|Player|GetPlayerPawn 0)))
  (Variables|Default|SetParent _asbp_loop_path))

(event Collision|EventActorBeginOverlap
  (params (OtherActor :type Actor%20Object%20Reference)))

(event EventTick
  (params (DeltaSeconds :type Float%20%28single-precision%29))
  (bind _returnvalue (Game|GetPlayerController 0))
  (bind (_worldlocation _worlddirection) (Game|Player|ConvertMouseLocationToWorldSpace _returnvalue))
  (if (Variables|Default|GetSelected)
    (bind _outhit (Collision|LineTraceByChannel _worldlocation (+ _worldlocation (* _worlddirection 1e+05)) "TraceTypeQuery1" false 0 "None"))
    (Transformation|SetActorLocation (Math|Vector|MakeVector (.X (Math|Vector|BreakVector (.Location (Collision|BreakHitResult _outhit)))) (.Y (Math|Vector|BreakVector (.Location (Collision|BreakHitResult _outhit)))) (.z (Transformation|GetActorLocation))) false false)
    (Spline|SetLocationatSplinePoint (Variables|/Game/LD47Custom/Blueprints/Characters/LoopPath/BP_LoopPath.BP_LoopPath_C|GetSpline (Variables|Default|GetParent)) (Variables|Default|GetOwningPointIndex) (Transformation|GetActorLocation) "World" true)
    (Development|PrintString (Utilities|String|ToString(Integer) (Variables|Default|GetOwningPointIndex)))))

(event EventRecieveSelection
  (Variables|Default|SetSelected true)
  (Transformation|DetachFromActor "KeepWorld" "KeepWorld" "KeepWorld"))

(event EventLoseSelection
  (Variables|Default|SetSelected false)
  (Transformation|AttachActorToActor (Variables|Default|GetParent) "None" "KeepWorld" "KeepWorld" "KeepWorld" true))

(fn ConstructionScript)