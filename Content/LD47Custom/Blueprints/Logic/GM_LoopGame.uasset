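; Game mode for the loop game that runs the music and restarts the current level after a win or when no BP_LoopFollower cultists remain.
; Music starts at BeginPlay or on the game instance's StartGame event, with an intro cue whose finish triggers the loop cue.
; Tick polls the follower count until a restart is pending, and both end conditions reopen the level through a delayed RestartMap timer.
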(event Custom|IntroFinished
  (Audio|PlaySound2D "/Game/LD47Custom/Audio/LD47lOOP_Cue.LD47lOOP_Cue" 1.0 1.0 0.0 0 0))

(event Custom|CustomEvent_0
  (bind _returnvalue (Audio|CreateSound2D "/Game/LD47Custom/Audio/LD47Intro_Cue.LD47Intro_Cue" 1.0 1.0 0.0 0))
  (EventDispatchers|BindEventtoOnAudioFinished _returnvalue (delegate Custom|IntroFinished))
  (Audio|Components|Audio|Play _returnvalue 0.0))

(event Custom|CustomEvent_1
  (Utilities|Time|SetTimerbyFunctionName 0 "RestartMap" 6.0))

(event EventBeginPlay
  (EventDispatchers|BindEventtoGameWon (delegate Custom|CustomEvent_1))
  (bind _asgi_loop_game (Utilities|Casting|CastToGI_LoopGame (Game|GetGameInstance)))
  (if (Variables|/Game/LD47Custom/Blueprints/Logic/GI_LoopGame.GI_LoopGame_C|GetGameStarted _asgi_loop_game)
    (bind _returnvalue (Audio|CreateSound2D "/Game/LD47Custom/Audio/LD47Intro_Cue.LD47Intro_Cue" 1.0 1.0 0.0 0))
    (EventDispatchers|BindEventtoOnAudioFinished _returnvalue (delegate Custom|IntroFinished))
    (Audio|Components|Audio|Play _returnvalue 0.0)
    (else
      (EventDispatchers|BindEventtoStartGame _asgi_loop_game (delegate Custom|CustomEvent_0)))))

(event EventTick
  (params (DeltaSeconds :type Float%20%28single-precision%29))
  (if (not (Variables|Default|GetPendingRestart))
    (CallFunction|CheckCultists)))

(fn ConstructionScript)

(fn CheckCultists
  (bind _outactors (Actor|GetAllActorsOfClass "/Game/LD47Custom/Blueprints/Characters/LoopFollower/BP_LoopFollower.BP_LoopFollower_C"))
  (if (<= (Utilities|Array|Length _outactors) 0)
    (Utilities|Time|SetTimerbyFunctionName 0 "RestartMap" 4.0)
    (Variables|Default|SetPendingRestart true)))

(fn RestartMap
  (bind _returnvalue (Game|GetCurrentLevelName true))
  (Game|OpenLevel(byName) (Utilities|String|StringToName _returnvalue)))