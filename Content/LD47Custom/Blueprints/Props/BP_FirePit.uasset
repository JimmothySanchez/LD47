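; BP_FirePit is a fire pit prop that can be lit once to spawn a loop follower AI.
; On BeginPlay it matches the visibility of its Niagara effect and point light to the Lit flag.
; The Light event, ignored if already lit, sets the flag, shows both components and spawns a BP_LoopFollower running its behavior tree at the Capsule's location.
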(event EventBeginPlay
  (Rendering|SetVisibility (Variables|Default|GetNiagara) (Variables|Default|GetLit) true)
  (Rendering|SetVisibility (Variables|Default|GetPointLight) (Variables|Default|GetLit) true))

(event Collision|EventActorBeginOverlap
  (params (OtherActor :type Actor%20Object%20Reference)))

(event EventTick
  (params (DeltaSeconds :type Float%20%28single-precision%29)))

(event EventLight
  (if (not (Variables|Default|GetLit))
    (Variables|Default|SetLit true)
    (Rendering|SetVisibility (Variables|Default|GetNiagara) (Variables|Default|GetLit) true)
    (Rendering|SetVisibility (Variables|Default|GetPointLight) (Variables|Default|GetLit) true)
    (AI|SpawnAIFromClass "/Game/LD47Custom/Blueprints/Characters/LoopFollower/BP_LoopFollower.BP_LoopFollower_C" "/Game/LD47Custom/Blueprints/Characters/LoopFollower/BT__LoopFollower.BT__LoopFollower" (Transformation|GetWorldLocation (Variables|Default|GetCapsule)) "0, 0, 0" false 0)))

(fn ConstructionScript)