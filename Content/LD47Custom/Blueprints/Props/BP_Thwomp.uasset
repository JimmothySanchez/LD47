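; BP_Thwomp is a crusher hazard prop whose mesh moves vertically and kills mortal actors it hits.
; On BeginPlay a timeline starts from StartTime, offsetting its phase, and drives the mesh's relative height scaled by MaxHeight.
; An event track on the timeline plays the impact sound at the actor's location.
; Movement is swept, and component hits send DieMessage to actors implementing I_Mortal.
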(event OnComponentHit(SM_Thwomp)
  (params (HitComponent :type Primitive%20Component%20Object%20Reference) (OtherActor :type Actor%20Object%20Reference) (OtherComp :type Primitive%20Component%20Object%20Reference) (NormalImpulse :type Vector :default "0, 0, 0") (Hit :type Hit%20Result%20Structure%20%28by%20ref%29))
  (if (Utilities|DoesObjectImplementInterface OtherActor "/Game/LD47Custom/Blueprints/Logic/I_Mortal.I_Mortal_C")
    (Class|IMortal|Die(Message) OtherActor)))

(event EventBeginPlay
  (Utilities|FlowControl|Sequence
    (:then_0
      (bind _thwompheight (Timeline|Timeline_0 SetNewTime)
        (:Update
          (Transformation|SetRelativeLocation (Variables|Default|GetSM_Thwomp) (Math|Vector|MakeVector 0.0 0.0 (* _thwompheight (Variables|Default|GetMaxHeight))) true false))
        (:NewTrack_0
          (Audio|PlaySoundatLocation "/Game/LD47Custom/Audio/Effects/Hit_Cue.Hit_Cue" (Transformation|GetActorLocation) "0, 0, 0" 1.0 1.0 0.0 0 0 0))))
    (:then_1
      (Timeline|Timeline_0 Play))))

(event Collision|EventActorBeginOverlap
  (params (OtherActor :type Actor%20Object%20Reference)))

(event EventTick
  (params (DeltaSeconds :type Float%20%28single-precision%29)))

(fn ConstructionScript)