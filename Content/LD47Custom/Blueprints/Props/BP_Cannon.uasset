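; BP_Cannon is a prop that fires BP_CannonProjectile actors from three muzzle points: left, top right and bottom right.
; On BeginPlay it seeks a timeline to StartTime and plays it, so each cannon's firing can be offset.
; The timeline's Fire event spawns a scaled-down projectile at each muzzle's world location and rotation.
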(event EventBeginPlay
  (bind _leftcannon (Variables|Default|GetLeftCannon))
  (bind _toprightcannon (Variables|Default|GetTopRightCannon))
  (bind _bottomrightcannon (Variables|Default|GetBottomRightCannon))
  (Utilities|FlowControl|Sequence
    (:then_0
      (Timeline|Timeline_0 SetNewTime
        (:Fire
          (Game|SpawnActorfromClass "/Game/LD47Custom/Blueprints/Props/BP_CannonProjectile.BP_CannonProjectile_C" (Math|Transform|MakeTransform (Transformation|GetWorldLocation _leftcannon) (Transformation|GetWorldRotation _leftcannon) "0.100000,0.100000,0.100000") "Undefined" 0 0)
          (Game|SpawnActorfromClass "/Game/LD47Custom/Blueprints/Props/BP_CannonProjectile.BP_CannonProjectile_C" (Math|Transform|MakeTransform (Transformation|GetWorldLocation _toprightcannon) (Transformation|GetWorldRotation _toprightcannon) "0.100000,0.100000,0.100000") "Undefined" 0 0)
          (Game|SpawnActorfromClass "/Game/LD47Custom/Blueprints/Props/BP_CannonProjectile.BP_CannonProjectile_C" (Math|Transform|MakeTransform (Transformation|GetWorldLocation _bottomrightcannon) (Transformation|GetWorldRotation _bottomrightcannon) "0.100000,0.100000,0.100000") "Undefined" 0 0))))
    (:then_1
      (Timeline|Timeline_0 Play))))

(event Collision|EventActorBeginOverlap
  (params (OtherActor :type Actor%20Object%20Reference)))

(event EventTick
  (params (DeltaSeconds :type Float%20%28single-precision%29)))

(fn ConstructionScript)